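; Game instance Blueprint that handles hosting, joining and leaving LAN multiplayer sessions.
; HostGameEvent creates a four-player session and opens MultiplayerLevel1 as a listen server, while LeaveGame destroys the session and opens Lobby, also as a listen server.
; JoinGame joins the first session found, or briefly shows a not-found message on BP_SessionJoiner text renders.
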(event Custom|HostGameEvent
  (|Session (Game|GetPlayerController 0) 4 true
    (:OnSuccess
      (Game|OpenLevel(byName) "MultiplayerLevel1" true "listen"))
    (:OnFailure
      (Development|PrintString "Something went bad"))))

(event Custom|LeaveGame
  (|DestroySession (Game|GetPlayerController 0)
    (:OnSuccess
      (Game|OpenLevel(byName) "Lobby" true "listen"))))

(event Custom|JoinGame
  (bind _results (|FindSessions (Game|GetPlayerController 0) 4 true)
    (:OnSuccess
      (if (== (Utilities|Array|Length _results) 0)
        (Development|PrintString "NoSessionsFound")
        (bind _outactors (Actor|GetAllActorsOfClass "/Game/BP_Solutions/BP_SessionJoiner.BP_SessionJoiner_C"))
        (for _array_element _outactors
          (Rendering|Components|TextRender|SetText (Variables|/Game/BP_Solutions/BP_SessionJoiner.BP_SessionJoiner_C|GetTextRender _array_element) "No Sesisons Found")
          (Utilities|FlowControl|Delay 3.0)
          (Rendering|Components|TextRender|SetText (Variables|/Game/BP_Solutions/BP_SessionJoiner.BP_SessionJoiner_C|GetTextRender _array_element) "Session Joiner"))
        (else
          (|JoinSession (Game|GetPlayerController 0) (Utilities|Array|Get(acopy) _results)))))))