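; Replication demo actor that shows a server-driven counter as in-world text using a RepNotify variable.
; On BeginPlay, only the authority starts a looping timer that calls UpdateCount to increment Count.
; OnRep_Count responds to each change by spawning an explosion emitter at CounterText and setting the text to the new value.
; Display updates ride on the notify, so Tick stays empty.
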(event EventBeginPlay
  (Networking|SwitchHasAuthority
    (:Authority
      (Utilities|Time|SetTimerbyFunctionName 0 "UpdateCount" 2.0 true))))

(event EventActorBeginOverlap
  (params (OtherActor :type Actor%20Object%20Reference)))

(event EventTick
  (params (DeltaSeconds :type Float%20%28single-precision%29))
  ;[1 1 1] Locally updates the text to reflect Server's Count
)

(fn ConstructionScript)

(fn UpdateCount
  (Variables|Default|SetCount (+ (Variables|Default|GetCount) 1)))

(fn OnRepCount
  (Effects|SpawnEmitteratLocation "/Game/StarterContent/Particles/P_Explosion.P_Explosion" (Transformation|GetWorldLocation (Variables|Default|GetCounterText)))
  (Rendering|Components|TextRender|SetText (Variables|Default|GetCounterText) (Utilities|String|ToString(Integer) (Variables|Default|GetCount))))